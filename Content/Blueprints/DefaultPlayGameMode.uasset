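; Gameplay game mode for the side-scroller that decides when a stage is cleared or the mission fails.
; BeginPlay caches the Boss-tagged actor, then Tick, while in Play, polls its state and the Paladin hero's death flag.
; Stage clear raises saved progress in the game instance and saves.
; Either outcome changes the gameplay state, shows its result widget and cursor, and disables player input.
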(event `self.ReceiveBeginPlay`
  ;[1 1 1] 스테이지 클리어
  (bind _outactors (`GameplayStatics.GetAllActorsWithTag` "Boss"))
  (bind _asboss_1monster_bp (cast `/Game/Blueprints/Boss1MonsterBP` (`|GetArrayItem` _outactors)))
  (set `self.Boss` _asboss_1monster_bp))

(event `self.ReceiveTick`
  (params (DeltaSeconds :type "Float (single-precision)"))
  (bind _returnvalue (`GameplayStatics.GetPlayerController` 0))
  (bind _returnvalue_2 (`GameplayStatics.GetPlayerController` 0))
  ;[1 1 1] 스테이지 클리어
  (switch `/Game/Enums/GamePlayState` (`self.CurGameplayState`)
    (:`NewEnumerator1`
      (if (`|EnumEquality` (`/Game/Blueprints/Boss1MonsterBP.CurState` (`self.Boss`)) "NewEnumerator4")
        (set `self.CurGameplayState` "NewEnumerator2")
        (bind _asside_scroll_game_instance (cast `/Game/Blueprints/SideScrollGameInstance` (`GameplayStatics.GetGameInstance`)))
        (bind _enterstage (`/Game/Blueprints/SideScrollGameInstance.EnterStage` _asside_scroll_game_instance))
        (if (> _enterstage (`/Game/Blueprints/SideScrollGameInstance.ClearStage` _asside_scroll_game_instance))
          (set `/Game/Blueprints/SideScrollGameInstance.ClearStage` _enterstage _asside_scroll_game_instance))
        (bind _returnvalue_3 (`|CreateWidget` "/Game/Blueprints/Widgets/StageClear.StageClear_C" _returnvalue))
        (`UserWidget.AddToViewport` _returnvalue_3 0)
        (set `PlayerController.bShowMouseCursor` true _returnvalue)
        (`self.DisableInput` (`GameplayStatics.GetPlayerCharacter` 0) (`GameplayStatics.GetPlayerController` 0))
        ;[1 1 1] 저장
        (bind _asside_scroll_game_instance_2 (cast `/Game/Blueprints/SideScrollGameInstance` (`GameplayStatics.GetGameInstance`)))
        (`/Game/Blueprints/SideScrollGameInstance.Save` _asside_scroll_game_instance_2)
        (else
          ;[1 1 1] 미션 실패
          (bind _aspaladin_hero_bp (cast `/Game/Blueprints/PaladinHeroBP` (`GameplayStatics.GetPlayerCharacter` 0)))
          (if (`/Game/Blueprints/PaladinHeroBP.isDeath` _aspaladin_hero_bp)
            (set `self.CurGameplayState` "NewEnumerator3")
            (bind _returnvalue_4 (`|CreateWidget` "/Game/Blueprints/Widgets/MissionFailed.MissionFailed_C" _returnvalue_2))
            (`UserWidget.AddToViewport` _returnvalue_4 0)
            (set `PlayerController.bShowMouseCursor` true _returnvalue_2)
            (`self.DisableInput` (`GameplayStatics.GetPlayerCharacter` 0) (`GameplayStatics.GetPlayerController` 0))))))))

(fn `UserConstructionScript`)