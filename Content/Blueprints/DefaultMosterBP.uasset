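; Base monster character, using a goblin death montage, that chases the player along the world Y axis.
; Each tick it caches Y-only distance and direction to the player, switching from Idle to Follow Char within range and then moving toward them without returning to Idle.
; Damage lowers Hp, briefly swaps the mesh material as a hit flash, and plays the death montage at zero, without stopping movement or destroying the actor.
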(event `self.ReceiveBeginPlay`)

(event `self.ReceiveTick`
  (params (DeltaSeconds :type "Float (single-precision)"))
  (`self.SaveDisAndDir`)
  (switch `/Game/Enums/MonsterState` (`self.CurState`)
    (:`NewEnumerator0`
      (if (<= (`self.DistancePlayerChar`) 500.0)
        (set `self.CurState` "NewEnumerator1")))
    (:`NewEnumerator1`
      (`self.AddMovementInput` (`self.DirToPlayerChar`)))))

(event `SaveDisAndDir`
  (bind _returnvalue (`KismetMathLibrary.MakeVector` 0.0 (.y (- (`self.K2_GetActorLocation` (`GameplayStatics.GetPlayerCharacter` 0)) (`self.K2_GetActorLocation`)))))
  (set `self.DistancePlayerChar` (`KismetMathLibrary.VSize` _returnvalue))
  (set `self.DirToPlayerChar` (`KismetMathLibrary.Normal` _returnvalue)))

(event `self.ReceiveAnyDamage`
  (params (Damage :type "Float (single-precision)") (DamageType :type "DamageType Object Reference") (InstigatedBy :type "Controller Object Reference") (DamageCauser :type "Actor Object Reference"))
  (bind _output_get (set `self.Hp` (- (`self.Hp`) Damage)))
  (`self.ChangeDamageColor`)
  (if (<= _output_get 0.0)
    (`self.PlayAnimMontage` "/Game/Mesh/Goblin/AnimMontage/goblin_death_Montage.goblin_death_Montage")))

(event `ChangeDamageColor`
  (`PrimitiveComponent.SetMaterial` (`self.Mesh`) 0 "/Game/Mesh/Goblin/phong1_Inst.phong1_Inst")
  (`KismetSystemLibrary.Delay` 0.2)
  (`PrimitiveComponent.SetMaterial` (`self.Mesh`) 0 "/Game/Mesh/Goblin/phong1.phong1"))

(fn `UserConstructionScript`)