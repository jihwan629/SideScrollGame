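; Stage 1 boss character that chases and attacks the Paladin hero along the Y axis, idling when the player dies or the stage clears.
; A Tick-driven state machine handles aggro, chase and attacks, while a self-recalling delay timer periodically swaps punches for a telegraphed swipe skill.
; Event hooks toggle sphere and capsule hitboxes that damage differently tagged characters.
; Incoming damage triggers hit flash, sound and sparks, then death montage and delayed destruction.
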(event `self.ReceiveBeginPlay`
  ;[1 1 1] 몬스터 행동 패턴
)

(event `SkillTimeLoop`
  ;[1 1 1] 스킬 타임 루프
  (`KismetSystemLibrary.Delay` 1.0)
  (set `self.SkillTime` (+ (`self.SkillTime`) 1.0))
  (`self.SkillTimeLoop`))

(event `self.ReceiveTick`
  (params (DeltaSeconds :type "Float (single-precision)"))
  ;[1 1 1] 몬스터 행동 패턴
  (`self.SaveDisAndDir`)
  (if (or (`self.isDeathPlayerChar`) (`self.isStageClear`))
    (set `self.CurState` "NewEnumerator3"))
  (switch `/Game/Enums/MonsterState` (`self.CurState`)
    (:`NewEnumerator0`
      (if (<= (`self.DistancePlayerChar`) 500.0)
        (set `self.CurState` "NewEnumerator1")
        (`self.SkillTimeLoop`)))
    (:`NewEnumerator1`
      (if (<= (`self.DistancePlayerChar`) 130.0)
        (`self.StartAttack`)
        (else
          (`self.AddMovementInput` (`self.DirToPlayerChar`)))))
    (:`NewEnumerator2`
      (if (`self.isAttacking`)
        _
        (elif (> (`self.DistancePlayerChar`) 150.0)
          (set `self.CurState` "NewEnumerator1"))))))

(event `SaveDisAndDir`
  (bind _returnvalue (`GameplayStatics.GetPlayerCharacter` 0))
  (bind _returnvalue_2 (`KismetMathLibrary.MakeVector` 0.0 (.y (- (`self.K2_GetActorLocation` _returnvalue) (`self.K2_GetActorLocation`)))))
  ;[1 1 1] 플레이어 정보 수집
  (bind _asdefault_play_game_mode (cast `/Game/Blueprints/DefaultPlayGameMode` (`GameplayStatics.GetGameMode`)))
  (set `self.isStageClear` (`|EnumEquality` (`/Game/Blueprints/DefaultPlayGameMode.CurGameplayState` _asdefault_play_game_mode) "NewEnumerator2"))
  (bind _aspaladin_hero_bp (cast `/Game/Blueprints/PaladinHeroBP` _returnvalue))
  (set `self.isDeathPlayerChar` (`/Game/Blueprints/PaladinHeroBP.isDeath` _aspaladin_hero_bp))
  (set `self.DistancePlayerChar` (`KismetMathLibrary.VSize` _returnvalue_2))
  (set `self.DirToPlayerChar` (`KismetMathLibrary.Normal` _returnvalue_2)))

(event `StartAttack`
  ;[1 1 1] 공격 시작
  (set `self.isAttacking` true)
  (if (>= (`self.SkillTime`) 10.0)
    (set `self.CurState` "NewEnumerator5")
    (`self.K2_SetActorRotation` (`KismetMathLibrary.Conv_VectorToRotator` (`self.DirToPlayerChar`)))
    (`PrimitiveComponent.SetMaterial` (`self.Mesh`) 0 "/Game/Mesh/Boss1/mutant_M_Skill_Inst.mutant_M_Skill_Inst")
    (set `self.SkillTime` 0.0)
    (`self.PlayAnimMontage` "/Game/Mesh/Boss1/AnimMongtages/mutant_flexing_muscles_Montage.mutant_flexing_muscles_Montage" 1.0 "Start")
    (`KismetSystemLibrary.Delay` 2.0)
    (`self.PlayAnimMontage` "/Game/Mesh/Boss1/AnimMongtages/mutant_swiping_Montage.mutant_swiping_Montage")
    (else
      (set `self.CurState` "NewEnumerator2")
      (`self.K2_SetActorRotation` (`KismetMathLibrary.Conv_VectorToRotator` (`self.DirToPlayerChar`)))
      (`self.PlayAnimMontage` "/Game/Mesh/Boss1/AnimMongtages/mutant_punch_Montage.mutant_punch_Montage"))))

(event `self.ReceiveAnyDamage`
  (params (Damage :type "Float (single-precision)") (DamageType :type "DamageType Object Reference") (InstigatedBy :type "Controller Object Reference") (DamageCauser :type "Actor Object Reference"))
  ;[1 1 1] 데미지 처리
  (bind _output_get (set `self.Hp` (- (`self.Hp`) Damage)))
  (`self.DamageEffect`)
  (if (<= _output_get 0.0)
    (`self.PlayAnimMontage` "/Game/Mesh/Boss1/AnimMongtages/mutant_dying_Montage.mutant_dying_Montage")
    (set `self.CurState` "NewEnumerator4")
    (`PrimitiveComponent.SetCollisionEnabled` (`self.CapsuleComponent`) "NoCollision")
    (`PrimitiveComponent.SetCollisionEnabled` (`self.Capsule`) "NoCollision")
    (`PrimitiveComponent.SetCollisionEnabled` (`self.Sphere`) "NoCollision")
    (`KismetSystemLibrary.Delay` 5.0)
    (`self.K2_DestroyActor`)))

(event `OnAnimEnd_Attack`
  ;[1 1 1] 공격 종료 후 행동 결정
  (`PrimitiveComponent.SetMaterial` (`self.Mesh`) 0 "/Game/Mesh/Boss1/mutant_M.mutant_M")
  (set `self.isAttacking` false)
  (if (or (`self.isDeathPlayerChar`) (`self.isStageClear`))
    (set `self.CurState` "NewEnumerator3")
    (elif (> (`self.DistancePlayerChar`) 180.0)
      (set `self.CurState` "NewEnumerator1")
      (else
        (`self.StartAttack`)))))

(event `DamageEffect`
  ;[1 1 1] 데미지 처리
  (`GameplayStatics.SpawnEmitterAttached` "/Game/InfinityBladeEffects/Effects/FX_Combat_Base/Impact/P_ImpactSpark.P_ImpactSpark" (`self.CapsuleComponent`))
  (`GameplayStatics.PlaySound2D` "/Game/Sounds_StrategyGame/Weapons/HandToHand/FightSword02_ImpactPound_Stereo.FightSword02_ImpactPound_Stereo" 0.4 1.0 0.0 null null)
  (`PrimitiveComponent.SetMaterial` (`self.Mesh`) 0 "/Game/Mesh/Boss1/mutant_M_Inst.mutant_M_Inst")
  (`KismetSystemLibrary.Delay` 0.2)
  (`PrimitiveComponent.SetMaterial` (`self.Mesh`) 0 "/Game/Mesh/Boss1/mutant_M.mutant_M"))

(event `self.Capsule.OnComponentBeginOverlap`
  (params (OverlappedComponent :type "PrimitiveComponent Object Reference") (OtherActor :type "Actor Object Reference") (OtherComp :type "PrimitiveComponent Object Reference") (OtherBodyIndex :type Integer) (bFromSweep :type Boolean) (SweepResult :type "HitResult Structure (by ref)"))
  ;[1 1 1] 공격 충돌 처리
  (if (!= OtherActor self)
    (if (!= (`|GetArrayItem` (`self.Tags`)) (`|GetArrayItem` (`Actor.Tags` OtherActor)))
      (if (== (`|GetArrayItem` (`ActorComponent.ComponentTags` OtherComp)) "Character")
        (`GameplayStatics.ApplyDamage` OtherActor (`self.Skill1Atk`) null self)))))

(event `self.Sphere.OnComponentBeginOverlap`
  (params (OverlappedComponent :type "PrimitiveComponent Object Reference") (OtherActor :type "Actor Object Reference") (OtherComp :type "PrimitiveComponent Object Reference") (OtherBodyIndex :type Integer) (bFromSweep :type Boolean) (SweepResult :type "HitResult Structure (by ref)"))
  ;[1 1 1] 공격 충돌 처리
  (if (!= OtherActor self)
    (if (!= (`|GetArrayItem` (`self.Tags`)) (`|GetArrayItem` (`Actor.Tags` OtherActor)))
      (if (== (`|GetArrayItem` (`ActorComponent.ComponentTags` OtherComp)) "Character")
        (`GameplayStatics.ApplyDamage` OtherActor (`self.Atk`) null self)))))

(event `OnColStart_Attack`
  ;[1 1 1] 공격 충돌 처리
  (`PrimitiveComponent.SetCollisionEnabled` (`self.Sphere`) "QueryAndPhysics"))

(event `OnColStart_Skill1Attack`
  ;[1 1 1] 공격 충돌 처리
  (`PrimitiveComponent.SetCollisionEnabled` (`self.Capsule`) "QueryAndPhysics"))

(event `OnColEnd_Attack`
  ;[1 1 1] 공격 충돌 처리
  (`PrimitiveComponent.SetCollisionEnabled` (`self.Sphere`) "NoCollision"))

(event `OnColEnd_Skill1Attack`
  ;[1 1 1] 공격 충돌 처리
  (`PrimitiveComponent.SetCollisionEnabled` (`self.Capsule`) "NoCollision"))

(fn `UserConstructionScript`)