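; Player-controlled Paladin character with a fixed-axis left/right move, jump, sword slash and health.
; Attack and jump play montages, and an IsAttacking flag blocks moving, jumping or re-attacking until the attack-end event.
; Collision start/end events toggle a hit capsule that damages overlapped character components whose actor tag differs.
; Incoming damage lowers Hp, briefly swaps the mesh material with a sound, and at zero plays death and disables input.
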(event `self.ReceiveBeginPlay`
  ;[1 1 1] 카메라
  (`PlayerController.SetViewTargetWithBlend` (`GameplayStatics.GetPlayerController` 0) (`self.Cam`) 0.0 "VTBlend_Linear" 0.0 false))

(event `Key|LeftMouseButton`
  (params (Key :type "Key Structure"))
  ;[1 1 1] 공격
  (:`Pressed`
    (if (not (`self.isAttacking`))
      (set `self.isAttacking` true)
      (`self.PlayAnimMontage` "/Game/Mesh/Paladin/AnimMontages/sword_and_shield_slash_Montage.sword_and_shield_slash_Montage"))))

(event `InputAxis|LeftRight`
  (params (AxisValue :type "Float (single-precision)"))
  ;[1 1 1] 이동
  (if (not (`self.isAttacking`))
    (`self.AddMovementInput` (0.0 1.0 0.0) AxisValue)))

(event `OnAnimEnd_Attack`
  ;[1 1 1] 공격
  (set `self.isAttacking` false))

(event `InputAxis|ForwardBackward`
  (params (AxisValue :type "Float (single-precision)"))
  ;[1 1 1] 이동
)

(event `Key|SpaceBar`
  (params (Key :type "Key Structure"))
  ;[1 1 1] 점프
  (:`Pressed`
    (if (`NavMovementComponent.IsFalling` (`self.CharacterMovement`))
      _
      (elif (not (`self.isAttacking`))
        (`self.Jump`)
        (`self.PlayAnimMontage` "/Game/Mesh/Paladin/AnimMontages/sword_and_shield_jump_Montage.sword_and_shield_jump_Montage"))))
  (:`Released`
    (`self.StopJumping`)))

(event `self.OnLanded`
  (params (Hit :type "HitResult Structure (by ref)"))
  ;[1 1 1] 점프
  (`self.StopAnimMontage` "/Game/Mesh/Paladin/AnimMontages/sword_and_shield_jump_Montage.sword_and_shield_jump_Montage"))

(event `self.Capsule.OnComponentBeginOverlap`
  (params (OverlappedComponent :type "PrimitiveComponent Object Reference") (OtherActor :type "Actor Object Reference") (OtherComp :type "PrimitiveComponent Object Reference") (OtherBodyIndex :type Integer) (bFromSweep :type Boolean) (SweepResult :type "HitResult Structure (by ref)"))
  ;[1 1 1] 공격 충돌 처리
  (if (== OtherActor self)
    _
    (elif (!= (`|GetArrayItem` (`self.Tags`)) (`|GetArrayItem` (`Actor.Tags` OtherActor)))
      (if (== (`|GetArrayItem` (`ActorComponent.ComponentTags` OtherComp)) "Character")
        (`GameplayStatics.ApplyDamage` OtherActor (`self.Atk`) null self)))))

(event `OnCollStart_Attack`
  ;[1 1 1] 공격 충돌 처리
  (`PrimitiveComponent.SetCollisionEnabled` (`self.Capsule`) "QueryAndPhysics"))

(event `OnCollEnd_Attack`
  ;[1 1 1] 공격 충돌 처리
  (`PrimitiveComponent.SetCollisionEnabled` (`self.Capsule`) "NoCollision"))

(event `self.ReceiveAnyDamage`
  (params (Damage :type "Float (single-precision)") (DamageType :type "DamageType Object Reference") (InstigatedBy :type "Controller Object Reference") (DamageCauser :type "Actor Object Reference"))
  ;[1 1 1] 데미지 처리
  (bind _output_get (set `self.Hp` (- (`self.Hp`) Damage)))
  (`self.ChangeDamageColor`)
  (if (<= _output_get 0.0)
    (`self.PlayAnimMontage` "/Game/Mesh/Paladin/AnimMontages/sword_and_shield_death_Montage.sword_and_shield_death_Montage")
    (set `self.isDeath` true)
    (`self.DisableInput` null)))

(event `ChangeDamageColor`
  ;[1 1 1] 데미지 처리
  (`GameplayStatics.PlaySound2D` "/Game/Sounds_ActionRPG/Creatures/Spider/A_Spider_Attack02.A_Spider_Attack02" 0.4 1.0 0.0 null null)
  (`PrimitiveComponent.SetMaterial` (`self.Mesh`) 0 "/Game/Mesh/Paladin/Paladin_MAT_Inst.Paladin_MAT_Inst")
  (`KismetSystemLibrary.Delay` 0.2)
  (`PrimitiveComponent.SetMaterial` (`self.Mesh`) 0 "/Game/Mesh/Paladin/Paladin_MAT.Paladin_MAT"))

(fn `UserConstructionScript`)