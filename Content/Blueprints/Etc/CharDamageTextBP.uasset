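; CharDamageTextBP is a floating damage number actor that shows an amount of damage as in-world text, then removes itself.
; SetDamageText floors the damage value and writes it to the TextRender component as a whole number.
; On BeginPlay a timeline offsets the text along world Z from the actor's start location, and the actor destroys itself when the timeline finishes.
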(event `self.ReceiveBeginPlay`
  ;[1 1 1] 텍스트 이동 후 삭제
  (set `self.StartPos` (`self.K2_GetActorLocation`))
  (bind (_direction _newtrack_0) (`Timeline|Timeline_0`)
    (:`Update`
      (`SceneComponent.K2_SetWorldLocation` (`self.TextRender`) (+ (`self.StartPos`) (`KismetMathLibrary.MakeVector` 0.0 0.0 (.x _newtrack_0))) false false))
    (:`Finished`
      (`self.K2_DestroyActor`))))

(fn `SetDamageText`
  (params (Damage :type "Float (double-precision)"))
  (`TextRenderComponent.K2_SetText` (`self.TextRender`) (`KismetTextLibrary.Conv_IntToText` (`KismetMathLibrary.FFloor` Damage))))

(fn `UserConstructionScript`)